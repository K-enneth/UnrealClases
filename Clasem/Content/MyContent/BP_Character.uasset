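; Player character with Enhanced Input movement, jump, look and toggleable pitch inversion, plus coin collection and danger-zone life drain.
; BeginPlay adds the input mapping context and shows the UWB_Test widget.
; Overlapping a BP_Item adds a point; any other actor sets the danger flag, which any end overlap clears.
; While flagged, Life drops a fixed amount per tick, frame-rate dependent; dispatchers broadcast point and life changes.
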(event Input|EnhancedActionEvents|EnhancedInputActionIA_MoveEx
  (params (ActionValue :type Vector%202D%20Structure) (ElapsedSeconds :type Float%20%28double-precision%29) (TriggeredSeconds :type Float%20%28double-precision%29) (InputAction :type Input%20Action%20Object%20Reference :default "/Game/MyContent/Inputs/IA_MoveEx.IA_MoveEx"))
  (bind _returnvalue (Pawn|GetControlRotation :!class /Script/Engine.Pawn))
  (Pawn|Input|AddMovementInput (Math|Vector|GetForwardVector (Math|Rotator|MakeRotator 0.0 0.0 (.yaw (Pawn|GetControlRotation :!class /Script/Engine.Pawn)))) (.y ActionValue) false)
  (Pawn|Input|AddMovementInput (Math|Vector|GetRightVector (Math|Rotator|MakeRotator (.roll _returnvalue) 0.0 (.yaw _returnvalue))) (.x ActionValue) false))

(event Input|EnhancedActionEvents|EnhancedInputActionIA_JumpEX
  (params (ActionValue :type Float%20%28double-precision%29) (ElapsedSeconds :type Float%20%28double-precision%29) (TriggeredSeconds :type Float%20%28double-precision%29) (InputAction :type Input%20Action%20Object%20Reference :default "/Game/MyContent/Inputs/IA_JumpEX.IA_JumpEX"))
  ;[1 1 1] Salto
  (Character|Jump))

(event Input|EnhancedActionEvents|EnhancedInputActionIA_LookEX
  (params (ActionValue :type Vector%202D%20Structure) (ElapsedSeconds :type Float%20%28double-precision%29) (TriggeredSeconds :type Float%20%28double-precision%29) (InputAction :type Input%20Action%20Object%20Reference :default "/Game/MyContent/Inputs/IA_LookEX.IA_LookEX"))
  (if (Variables|Default|GetIsInverse)
    (Pawn|Input|AddControllerPitchInput (.y ActionValue))
    (else
      (Pawn|Input|AddControllerPitchInput (* (.y ActionValue) -1.0))))
  (Pawn|Input|AddControllerYawInput (.x ActionValue)))

(event Input|EnhancedActionEvents|EnhancedInputActionIA_ChangeAxis
  (params (ActionValue :type Boolean) (ElapsedSeconds :type Float%20%28double-precision%29) (TriggeredSeconds :type Float%20%28double-precision%29) (InputAction :type Input%20Action%20Object%20Reference :default "/Game/MyContent/Inputs/IA_ChangeAxis.IA_ChangeAxis"))
  (Variables|Default|SetIsInverse (not (Variables|Default|GetIsInverse))))

(event EventBeginPlay
  (Utilities|FlowControl|Sequence
    (:then_0
      (Input|AddMappingContext (PlayerController|LocalPlayerSubsystems|GetEnhancedInputLocalPlayerSubsystem (Game|GetPlayerController 0)) "/Game/MyContent/Inputs/IMC_Example.IMC_Example" 0 "(bIgnoreAllPressedKeysUntilRelease=True,bForceImmediately=False,bNotifyUserSettings=False)"))
    (:then_1
      (Variables|Default|SetStartPos "0, 0, 0"))
    (:then_2
      (bind _returnvalue (UserInterface|CreateWidget "/Game/MyContent/Widget/UWB_Test.UWB_Test_C"))
      (UserInterface|Viewport|AddtoViewport _returnvalue 0))))

(event Collision|EventActorEndOverlap
  (params (OtherActor :type Actor%20Object%20Reference))
  (Variables|Default|SetisInDangerZone false))

(event Collision|EventActorBeginOverlap
  (params (OtherActor :type Actor%20Object%20Reference))
  (Utilities|Casting|CastToBP_Item OtherActor
    (:then
      (bind _result (Math|Integer|IncrementInt (Variables|Default|GetPoints))
        (:%20%20
          (Default|CallOnCoinCollected _result))))
    (:CastFailed
      (Variables|Default|SetisInDangerZone true))))

(event EventTick
  (params (DeltaSeconds :type Float%20%28single-precision%29))
  (if (Variables|Default|GetisInDangerZone)
    (bind _output_get (Variables|Default|SetLife (- (Variables|Default|GetLife) 0.01)))
    (Default|CallOnLifeSubstracted _output_get)))

(fn ConstructionScript)