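; BP_Generator is an actor that loads grid data from a JSON file when play begins; no spawning or generation is implemented.
; It stores the file's rows, cols and matrix fields in variables, then runs a nested row and column loop.
; The loop only prints a default debug string per cell, as the flattened-index Matrix lookup is left unused alongside disconnected test prints.
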(event EventBeginPlay
  ;[0.7047 0.6108 1] Read from Json
  (bind _outjsonobject (Class|JsonBlueprintFunctionLibrary|FromFile (Variables|Default|GetOtherFile)))
  (Utilities|FlowControl|Sequence
    (:then_0
      (bind _outvalue (|GetJsonField _outjsonobject "rows"))
      (Variables|Default|Setrows _outvalue))
    (:then_1
      (bind _outvalue_2 (|GetJsonField _outjsonobject "cols"))
      (Variables|Default|Setcols _outvalue_2))
    (:then_2
      (bind _outvalue_3 (|GetJsonField _outjsonobject "matrix"))
      (Variables|Default|Setmatrix _outvalue_3))
    (:then_3
      (for _index (range 0 (- (Variables|Default|Getrows) 1))
        (for _index_2 (range 0 (- (Variables|Default|Getcols) 1))
          (Development|PrintString "Hello" true true "(R=0.000000,G=0.660000,B=1.000000,A=1.000000)" 1e+01))))))

(fn ConstructionScript)