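; BP_Generator is an actor that procedurally builds a room layout from a JSON file when play begins.
; It reads row and column counts plus a flat matrix of room IDs from the file.
; A nested loop walks the matrix as a grid, skipping zero cells.
; Each other value, less one, indexes the Rooms class array, and that room spawns on a fixed-spacing grid.
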(event EventBeginPlay
  ;[0.7047 0.6108 1] Read from Json
  (bind _outjsonobject (Class|JsonBlueprintFunctionLibrary|FromFile (Variables|Default|GetOtherFile)))
  (Utilities|FlowControl|Sequence
    (:then_0
      (bind _outvalue (|GetJsonField _outjsonobject "rows"))
      (Variables|Default|Setrows _outvalue))
    (:then_1
      (bind _outvalue_2 (|GetJsonField _outjsonobject "cols"))
      (Variables|Default|Setcols _outvalue_2))
    (:then_2
      (bind _outvalue_3 (|GetJsonField _outjsonobject "matrix"))
      (Variables|Default|Setmatrix _outvalue_3))
    (:then_3
      (Variables|Default|SetCounter 0)
      (for _index (range 0 (- (Variables|Default|Getrows) 1))
        (for _index_2 (range 0 (- (Variables|Default|Getcols) 1))
          (bind _result (Math|Integer|IncrementInt (Variables|Default|GetCounter))
            (:%20%20
              (if (!= (Utilities|Array|Get(acopy) (Variables|Default|Getmatrix) (- _result 1)) 0)
                (bind _result_2 (Math|Integer|DecrementInt (Utilities|Array|Get(acopy) (Variables|Default|Getmatrix) (- _result 1)))
                  (:%20%20
                    (bind _output_get (Variables|Default|SetSpawn (Math|Transform|MakeTransform (Math|Vector|MakeVector (Math|Conversions|ToFloat(Integer) (* _index 402)) (Math|Conversions|ToFloat(Integer) (* _index_2 402)) 0.0) "0, 0, 0" "1.000000,1.000000,1.000000")))
                    (Game|SpawnActorfromClass (Utilities|Array|Get(acopy) (Variables|Default|GetRooms) _result_2) _output_get "Undefined" "MultiplyWithRoot" 0 0)))))))))))

(fn ConstructionScript)