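; BP_Room9 is a procedural room actor that serves as the win condition when the player enters it.
; On overlap with BP_ThirdPersonCharacter, it checks whether the character has obtained at least two items.
; If so, it shows the BPW_Win widget and disables player input; otherwise it prints a missing-items message.
; BeginPlay and the construction script only call the parent versions, and Tick is disabled.
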(event Collision|EventActorBeginOverlap
  (params (OtherActor :type Actor%20Object%20Reference))
  (bind _returnvalue (Game|GetPlayerController 0))
  (bind _asbp_third_person_character (Utilities|Casting|CastToBP_ThirdPersonCharacter OtherActor))
  (if (>= (Variables|/Game/ThirdPerson/Blueprints/BP_ThirdPersonCharacter.BP_ThirdPersonCharacter_C|GetItemsObtained _asbp_third_person_character) 2)
    (bind _returnvalue_2 (UserInterface|CreateWidget "/Game/MyContent/Actors/Procedural/Widgets/BPW_Win.BPW_Win_C" _returnvalue))
    (UserInterface|Viewport|AddtoViewport _returnvalue_2 0)
    (Input|DisableInput (Game|GetPlayerCharacter 0) _returnvalue)
    (else
      (Development|PrintString "Faltan Items"))))

(event EventTick
  (params (DeltaSeconds :type Float%20%28single-precision%29))
  (|CallParentFunction DeltaSeconds) ; This node is disabled and will not be called.\nDrag off pins to build functionality.
)

(event EventBeginPlay
  (|CallParentFunction))

(fn ConstructionScript
  (|CallParentFunction))